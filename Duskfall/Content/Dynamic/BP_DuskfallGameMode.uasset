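; Game mode for Duskfall that runs boss fights, checkpoints, player respawn and pausing.
; On BeginPlay it updates the game instance state and records every AI enemy's spawn location in a map.
; Boss events show or remove the health bar and message tagged entrance and exit doors.
; Respawn teleports the player to the current checkpoint, returns surviving enemies to their recorded locations with healing, and resets the church boss's state.
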(event EventCheckPointHint
  (params (Checkpoint :type Check%20Point%20Object%20Reference))
  (Variables|Default|SetCurrentCheckPoint Checkpoint))

(event EventRespawnPlayer
  (params (Character :type Character%20Object%20Reference))
  (CallFunction|SetPlayertoCheckPoint Character)
  (CallFunction|ResetAllRemainingEnemies)
  (bind _aschurch_boss_enemy (Utilities|Casting|CastToChurchBossEnemy (Variables|Default|GetBoss)))
  (Variables|/Game/Dynamic/Characters/AI/ChurchBossEnemy.ChurchBossEnemy_C|SetBossState _aschurch_boss_enemy "NewEnumerator0"))

(event EventBeginPlay
  (bind _asbp_game_instance (Utilities|Casting|CastToBP_GameInstance (Game|GetGameInstance)))
  (Default|UpdateGameState _asbp_game_instance "NewEnumerator4")
  (bind _outactors (Actor|GetAllActorsOfClass "/Script/Duskfall.BaseAICharacter"))
  (for _array_element _outactors
    (Utilities|Map|Add (Variables|Default|GetEnemeies) _array_element (Transformation|GetActorLocation _array_element))))

(event EventPauseGame
  (params (Controller :type Player%20Controller%20Object%20Reference))
  (Variables|Default|SetPlayerWhoPuased Controller)
  (bind _returnvalue (UserInterface|CreateWidget "/Game/Dynamic/UI/WBP_PauseMenu.WBP_PauseMenu_C" Controller))
  (bind _output_get (Variables|Default|SetPauseMenu _returnvalue))
  (UserInterface|Viewport|AddtoViewport _output_get 0)
  (Input|SetInputModeUIOnly Controller (Variables|/Game/Dynamic/UI/WBP_PauseMenu.WBP_PauseMenu_C|GetResumeButton _output_get) "DoNotLock")
  (Game|SetGamePaused true))

(event EventResumeGame
  (params (Controller :type Player%20Controller%20Object%20Reference))
  (Widget|RemovefromParent (Variables|Default|GetPauseMenu))
  (Input|SetInputModeGameOnly (Variables|Default|GetPlayerWhoPuased))
  (Game|SetGamePaused false))

(event EventBossFightStart
  (params (Boss :type Duskfall%20Character%20Object%20Reference))
  (bind _output_get (Variables|Default|SetBoss Boss))
  (CallFunction|AddBossUI _output_get)
  (bind _outactors (Actor|GetAllActorsOfClass "/Game/Dynamic/Terrain/Puzzle/BP_StandardDoor.BP_StandardDoor_C"))
  (for _array_element _outactors
    (if (Utilities|Array|ContainsItem (Variables|/Script/Engine.Actor|GetTags _array_element) "BossEntrance")
      (Class|IInteractable|Turnon(Message) _array_element))))

(event EventBossFightReset
  (Widget|RemovefromParent (Variables|Default|GetBossHealthBar))
  (bind _outactors (Actor|GetAllActorsOfClass "/Game/Dynamic/Terrain/Puzzle/BP_StandardDoor.BP_StandardDoor_C"))
  (for _array_element _outactors
    (if (Utilities|Array|ContainsItem (Variables|/Script/Engine.Actor|GetTags _array_element) "BossEntrance")
      (Class|IInteractable|TurnOff(Message) _array_element))))

(event EventBossFightComplete
  (Widget|RemovefromParent (Variables|Default|GetBossHealthBar))
  (bind _outactors (Actor|GetAllActorsOfClass "/Game/Dynamic/Terrain/Puzzle/BP_StandardDoor.BP_StandardDoor_C"))
  (for _array_element _outactors
    (if (Utilities|Array|ContainsItem (Variables|/Script/Engine.Actor|GetTags _array_element) "BossExit")
      (Class|IInteractable|Turnon(Message) _array_element))))

(event EventPlayerDeath
  (Utilities|IsValid (Variables|Default|GetBoss)
    (:Is%20Valid
      (CallFunction|BossFightReset)
      (bind _aschurch_boss_enemy (Utilities|Casting|CastToChurchBossEnemy (Variables|Default|GetBoss)))
      (Variables|/Game/Dynamic/Characters/AI/ChurchBossEnemy.ChurchBossEnemy_C|SetBossState _aschurch_boss_enemy "NewEnumerator8"))))

(fn ConstructionScript)

(fn SetPlayertoCheckPoint
  (params (Character :type Character%20Object%20Reference))
  (Transformation|SetWorldLocation (Variables|/Script/Engine.Character|GetCapsuleComponent Character) (Transformation|GetWorldLocation (Variables|/Game/Dynamic/Terrain/CheckPoint.CheckPoint_C|GetDefaultSceneRoot (Variables|Default|GetCurrentCheckPoint))) false true))

(fn ResetAllRemainingEnemies
  (bind _enemeies (Variables|Default|GetEnemeies))
  (bind _keys (Utilities|Map|Keys _enemeies))
  (for _array_element _keys
    (Utilities|IsValid _array_element
      (:Is%20Valid
        (Transformation|SetActorLocation _array_element (.Value (Utilities|Map|Find _enemeies _array_element)) false true)
        (Class|HealthSystem|GainHealth(Message) _array_element 5e+02 self)))))

(fn AddBossUI
  (params (User :type Duskfall%20Character%20Object%20Reference))
  (bind _returnvalue (UserInterface|CreateWidget "/Game/Dynamic/UI/WBP_BossHealthBar.WBP_BossHealthBar_C" (Game|GetPlayerController 0)))
  (Variables|Default|SetBossHealthBar _returnvalue)
  (UserInterface|Viewport|AddtoViewport _returnvalue 0)
  (Default|SetUser _returnvalue User))