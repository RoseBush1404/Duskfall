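; Player character Blueprint that handles using switches and the death and respawn sequence.
; UsePressed runs a near-stationary box trace around the muzzle point and sends SwitchMessage to every hit actor.
; Die, guarded by IsDead, notifies the game mode, fades the camera and disables input.
; After timed delays it requests a respawn through the game mode, restores health, then reverses the fade and re-enables input.
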(event EventUsePressed
  (bind _muzzlepoint (Variables|Default|GetMuzzlePoint))
  (bind _returnvalue (Transformation|GetWorldRotation _muzzlepoint))
  (bind _returnvalue_2 (Transformation|GetWorldLocation _muzzlepoint))
  (bind _returnvalue_3 (Math|Vector|RotateVector "-25.000000, 0, 0" _returnvalue))
  (bind _returnvalue_4 (+ _returnvalue_2 _returnvalue_3))
  (bind _outhits (Class|KismetSystemLibrary|BoxTraceMulti _returnvalue_4 (+ _returnvalue_4 1) "50.000000,50.000000,50.000000" _returnvalue "TraceTypeQuery1" false 0 "None" true))
  (bind _array_element (Utilities|Array|ForEachLoopwithBreak _outhits)
    (:LoopBody
      (Class|IInteractable|Switch(Message) (.HitActor (Collision|BreakHitResult _array_element))))))

(event EventDie
  (if (not (Variables|Default|GetIsDead))
    (bind _asbp_player_controller (Utilities|Casting|CastToBP_PlayerController (Game|GetPlayerController 0)))
    (Class|IGameMode|PlayerDeath(Message) (Game|GetGameMode))
    (Default|CameraFadein _asbp_player_controller)
    (Input|DisableInput _asbp_player_controller _asbp_player_controller)
    (Variables|Default|SetIsDead true)
    (Utilities|FlowControl|Delay 2.0)
    (Class|IGameMode|RespawnPlayer(Message) (Game|GetGameMode) self)
    (Class|DuskfallCharacter|GainHealth 5e+02 self)
    (Utilities|FlowControl|Delay 2.0)
    (Default|CameraFadeOut _asbp_player_controller)
    (Input|EnableInput _asbp_player_controller _asbp_player_controller)
    (Variables|Default|SetIsDead false)))

(fn ConstructionScript)