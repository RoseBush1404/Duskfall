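; Player controller that routes player input to the controlled pawn and handles pause and camera fade.
; Movement, turn and action inputs (jump, attack, block, dash, use) are forwarded as messages to whatever valid pawn is possessed, keeping gameplay logic out of the controller.
; Pause toggles through game mode messages.
; CameraFadeIn and CameraFadeOut run one timeline forward or reversed, driving the UI's on-screen alpha.
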(event Custom|CameraFadeOut
  (bind _ui (Variables|Default|GetUI))
  (bind _alpha (Timeline|Timeline_0 ReverseFromEnd)
    (:Update
      (Utilities|IsValid _ui
        (:Is%20Valid
          (Default|SetAlphaonScreen _ui _alpha))))))

(event Custom|CameraFadeIn
  (bind _ui (Variables|Default|GetUI))
  (bind _alpha (Timeline|Timeline_0 PlayFromStart)
    (:Update
      (Utilities|IsValid _ui
        (:Is%20Valid
          (Default|SetAlphaonScreen _ui _alpha))))))

(event EventBeginPlay)

(event Input|ActionEvents|InputActionJump
  (params (Key :type Key%20Structure :default "None"))
  (bind _returnvalue (Pawn|GetControlledPawn))
  (:Pressed
    (Utilities|IsValid _returnvalue
      (:Is%20Valid
        (Class|CharacterControls|JumpPressed(Message) _returnvalue))))
  (:Released
    (Utilities|IsValid _returnvalue
      (:Is%20Valid
        (Class|CharacterControls|JumpReleased(Message) _returnvalue)))))

(event Input|ActionEvents|InputActionAttack
  (params (Key :type Key%20Structure :default "None"))
  (bind _returnvalue (Pawn|GetControlledPawn))
  (:Pressed
    (Utilities|IsValid _returnvalue
      (:Is%20Valid
        (Class|CharacterControls|AttackPressed(Message) _returnvalue))))
  (:Released
    (Utilities|IsValid _returnvalue
      (:Is%20Valid
        (Class|CharacterControls|AttackReleased(Message) _returnvalue)))))

(event Input|ActionEvents|InputActionBlock
  (params (Key :type Key%20Structure :default "None"))
  (bind _returnvalue (Pawn|GetControlledPawn))
  (:Pressed
    (Utilities|IsValid _returnvalue
      (:Is%20Valid
        (Class|CharacterControls|BlockPressed(Message) _returnvalue))))
  (:Released
    (Utilities|IsValid _returnvalue
      (:Is%20Valid
        (Class|CharacterControls|BlockReleased(Message) _returnvalue)))))

(event Input|ActionEvents|InputActionDash
  (params (Key :type Key%20Structure :default "None"))
  (bind _returnvalue (Pawn|GetControlledPawn))
  (:Pressed
    (Utilities|IsValid _returnvalue
      (:Is%20Valid
        (Class|CharacterControls|DashPressed(Message) _returnvalue))))
  (:Released
    (Utilities|IsValid _returnvalue
      (:Is%20Valid
        (Class|CharacterControls|DashReleased(Message) _returnvalue)))))

(event Input|ActionEvents|InputActionUse
  (params (Key :type Key%20Structure :default "None"))
  (bind _returnvalue (Pawn|GetControlledPawn))
  (:Pressed
    (Utilities|IsValid _returnvalue
      (:Is%20Valid
        (Class|CharacterControls|UsePressed(Message) _returnvalue))))
  (:Released
    (Utilities|IsValid _returnvalue
      (:Is%20Valid
        (Class|CharacterControls|UseReleased(Message) _returnvalue)))))

(event Input|ActionEvents|InputActionPause
  (params (Key :type Key%20Structure :default "None"))
  (bind _returnvalue (Game|GetGameMode))
  (bind _self self)
  (:Pressed
    (if (Game|IsGamePaused)
      (Class|IGameMode|ResumeGame(Message) _returnvalue _self)
      (else
        (Class|IGameMode|PauseGame(Message) _returnvalue _self)))))

(event Input|AxisEvents|InputAxisMoveForward
  (params (AxisValue :type Float%20%28single-precision%29))
  (bind _returnvalue (Pawn|GetControlledPawn))
  (Utilities|IsValid _returnvalue
    (:Is%20Valid
      (Class|CharacterControls|MoveForward(Message) _returnvalue AxisValue))))

(event Input|AxisEvents|InputAxisMoveRight
  (params (AxisValue :type Float%20%28single-precision%29))
  (bind _returnvalue (Pawn|GetControlledPawn))
  (Utilities|IsValid _returnvalue
    (:Is%20Valid
      (Class|CharacterControls|MoveRight(Message) _returnvalue AxisValue))))

(event Input|AxisEvents|InputAxisTurn
  (params (AxisValue :type Float%20%28single-precision%29))
  (bind _returnvalue (Pawn|GetControlledPawn))
  (Utilities|IsValid _returnvalue
    (:Is%20Valid
      (Class|CharacterControls|Turn(Message) _returnvalue AxisValue))))

(event Input|AxisEvents|InputAxisTurnRate
  (params (AxisValue :type Float%20%28single-precision%29))
  (bind _returnvalue (Pawn|GetControlledPawn))
  (Utilities|IsValid _returnvalue
    (:Is%20Valid
      (Class|CharacterControls|TurnRate(Message) _returnvalue AxisValue))))

(fn ConstructionScript)