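; Player controller that relays player input to whichever pawn it currently controls.
; Jump, Attack, Block and Dash press and release events, plus movement and turn axes, each forward a matching message to the controlled pawn.
; The message calls decouple input from any specific pawn class, leaving each pawn to decide how to respond.
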(event Input|ActionEvents|InputActionJump
  (params (Key :type Key%20Structure))
  (bind _returnvalue (Pawn|GetControlledPawn))
  (:Pressed
    (Class|CharacterControls|JumpPressed(Message) _returnvalue))
  (:Released
    (Class|CharacterControls|JumpReleased(Message) _returnvalue)))

(event Input|ActionEvents|InputActionAttack
  (params (Key :type Key%20Structure))
  (bind _returnvalue (Pawn|GetControlledPawn))
  (:Pressed
    (Class|CharacterControls|AttackPressed(Message) _returnvalue))
  (:Released
    (Class|CharacterControls|AttackReleased(Message) _returnvalue)))

(event Input|ActionEvents|InputActionBlock
  (params (Key :type Key%20Structure))
  (bind _returnvalue (Pawn|GetControlledPawn))
  (:Pressed
    (Class|CharacterControls|BlockPressed(Message) _returnvalue))
  (:Released
    (Class|CharacterControls|BlockReleased(Message) _returnvalue)))

(event Input|ActionEvents|InputActionDash
  (params (Key :type Key%20Structure))
  (bind _returnvalue (Pawn|GetControlledPawn))
  (:Pressed
    (Class|CharacterControls|DashPressed(Message) _returnvalue))
  (:Released
    (Class|CharacterControls|DashReleased(Message) _returnvalue)))

(event Input|AxisEvents|InputAxisMoveForward
  (params (AxisValue :type Float%20%28single-precision%29))
  (Class|CharacterControls|MoveForward(Message) (Pawn|GetControlledPawn) AxisValue))

(event Input|AxisEvents|InputAxisMoveRight
  (params (AxisValue :type Float%20%28single-precision%29))
  (Class|CharacterControls|MoveRight(Message) (Pawn|GetControlledPawn) AxisValue))

(event Input|AxisEvents|InputAxisTurn
  (params (AxisValue :type Float%20%28single-precision%29))
  (Class|CharacterControls|Turn(Message) (Pawn|GetControlledPawn) AxisValue))

(event Input|AxisEvents|InputAxisTurnRate
  (params (AxisValue :type Float%20%28single-precision%29))
  (Class|CharacterControls|TurnRate(Message) (Pawn|GetControlledPawn) AxisValue))

(fn ConstructionScript)