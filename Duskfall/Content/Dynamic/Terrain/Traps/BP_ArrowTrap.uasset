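; BP_ArrowTrap is a trap that spawns projectiles from its Arrow component's transform, with itself as owner.
; A timer drives firing at the configured rate and looping setting, starting on BeginPlay when IsOn is set or through the Turnon event, and cleared by TurnOff.
; Each spawned projectile receives the trap's damage amount and a fixed, neutral damage modifier.
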(event Custom|Fire
  (bind _returnvalue (Game|SpawnActorfromClass (Variables|Default|GetProjectile) (Transformation|GetWorldTransform (Variables|Default|GetArrow)) "Undefined" self 0))
  (Variables|/Script/Duskfall.DuskfallProjectile|SetDamageAmount _returnvalue (Variables|Default|GetDamage))
  (Variables|/Script/Duskfall.DuskfallProjectile|SetDamageModifer _returnvalue 1.0))

(event EventTurnon
  (bind _returnvalue (Utilities|Time|SetTimerbyEvent (delegate Custom|Fire) (Variables|Default|GetFireRate) (Variables|Default|GetLooping)))
  (Variables|Default|SetFiringTimer _returnvalue))

(event EventTurnOff
  (Utilities|Time|ClearandInvalidateTimerbyHandle (Variables|Default|GetFiringTimer)))

(event EventBeginPlay
  (if (Variables|Default|GetIsOn)
    (bind _returnvalue (Utilities|Time|SetTimerbyEvent (delegate Custom|Fire) (Variables|Default|GetFireRate) (Variables|Default|GetLooping)))
    (Variables|Default|SetFiringTimer _returnvalue)))

(fn ConstructionScript)