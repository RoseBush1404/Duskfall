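; BP_Switch is a 2D switch that toggles linked devices on and off.
; Its Switch event flips IsOn, swaps the on or off flipbook, prints a debug string and sends TurnOnMessage or TurnOffMessage to every entry in Devices.
; An optional single-use flag blocks further toggles after the first.
; The construction script sets the flipbook to match the initial IsOn state.
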(event EventSwitch
  (bind _paperflipbook (Variables|Default|GetPaperFlipbook))
  (bind _devices (Variables|Default|GetDevices))
  (if (Variables|Default|GetCanBeUsedOnes)
    (if (not (Variables|Default|GetBeenUsed))
      (Variables|Default|SetBeenUsed true)
      (if (Variables|Default|GetIsOn) :!label _label
        (Variables|Default|SetIsOn false)
        (Sprite|SetFlipbook _paperflipbook (Variables|Default|GetOffSprite))
        (Development|PrintString "turnning off")
        (bind _array_element (Utilities|Array|ForEachLoopwithBreak _devices)
          (:LoopBody
            (Class|IInteractable|TurnOff(Message) _array_element)))
        (else
          (Variables|Default|SetIsOn true)
          (Sprite|SetFlipbook _paperflipbook (Variables|Default|GetOnSprite))
          (Development|PrintString "turnning on")
          (bind _array_element_2 (Utilities|Array|ForEachLoopwithBreak _devices)
            (:LoopBody
              (Class|IInteractable|Turnon(Message) _array_element_2))))))
    (else
      (goto _label))))

(fn ConstructionScript
  (bind _paperflipbook (Variables|Default|GetPaperFlipbook))
  (if (Variables|Default|GetIsOn)
    (Sprite|SetFlipbook _paperflipbook (Variables|Default|GetOnSprite))
    (else
      (Sprite|SetFlipbook _paperflipbook (Variables|Default|GetOffSprite)))))