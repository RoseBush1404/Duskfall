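; BP_SwitchBox is a trigger box that switches a list of devices on or off when the player character overlaps it.
; On overlap it sends either a turn-on or turn-off message to every entry in Devices, as chosen by TurnDevicesOn.
; An optional single-use flag limits it to firing once; otherwise it fires on every overlap.
; The construction script sizes the box from BoxBounds.
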(event OnComponentBeginOverlap(Box)
  (params (OverlappedComponent :type Primitive%20Component%20Object%20Reference) (OtherActor :type Actor%20Object%20Reference) (OtherComp :type Primitive%20Component%20Object%20Reference) (OtherBodyIndex :type Integer) (bFromSweep :type Boolean) (SweepResult :type Hit%20Result%20Structure%20%28by%20ref%29))
  (bind _devices (Variables|Default|GetDevices))
  (bind _asbp_player_character (Utilities|Casting|CastToBP_PlayerCharacter OtherActor))
  (Utilities|IsValid _asbp_player_character
    (:Is%20Valid
      (if (Variables|Default|GetCanBeUsedOnes)
        (if (not (Variables|Default|GetBeenUsed))
          (Variables|Default|SetBeenUsed true)
          (if (Variables|Default|GetTurnDevicesOn) :!label _label
            (for _array_element _devices
              (Class|IInteractable|Turnon(Message) _array_element))
            (else
              (for _array_element_2 _devices
                (Class|IInteractable|TurnOff(Message) _array_element_2)))))
        (else
          (goto _label))))))

(fn ConstructionScript
  (Components|Box|SetBoxExtent (Variables|Default|GetBox) (Variables|Default|GetBoxBounds) true))