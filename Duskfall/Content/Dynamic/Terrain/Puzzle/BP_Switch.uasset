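; BP_Switch is a puzzle switch with on and off flipbooks that sends turn-on or turn-off messages to an array of Devices.
; Switch toggles the state with a slide sound and can be limited to a single use.
; In timer mode it blocks further use and plays a timer sound until a timer reverts the state, re-enables it and destroys the sound.
; The construction script previews the initial state's flipbook.
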(event EventSwitch
  (bind _returnvalue (Transformation|GetActorLocation))
  (bind _istimertoggled (Variables|Default|GetIsTimerToggled))
  (bind _toggletime (Variables|Default|GetToggleTime))
  (if (Variables|Default|GetCanBeUsed)
    (if (Variables|Default|GetCanBeUsedOnes)
      (if (not (Variables|Default|GetBeenUsed))
        (Variables|Default|SetBeenUsed true)
        (if (Variables|Default|GetIsOn) :!label _label
          (Audio|PlaySoundatLocation "/Game/Static/Audio/Puzzle/Slide_2_Cue.Slide_2_Cue" _returnvalue "0, 0, 0" 1.0 1.0 0.0 0 0 0)
          (CallFunction|TurnOffDevices)
          (if _istimertoggled
            (Utilities|Time|SetTimerbyFunctionName 0 "TurnOnDevices" _toggletime)
            (Variables|Default|SetCanBeUsed false)
            (bind _returnvalue_2 (Audio|SpawnSoundatLocation "/Game/Static/Audio/Puzzle/Ladder_2_Cue.Ladder_2_Cue" (Transformation|GetActorLocation) "0, 0, 0" 0.8 1.0 0.0 0 0 false :!label _label_2))
            (Variables|Audio|SetTimerSounc _returnvalue_2))
          (else
            (Audio|PlaySoundatLocation "/Game/Static/Audio/Puzzle/Slide_2_Cue.Slide_2_Cue" _returnvalue "0, 0, 0" 1.0 1.0 0.0 0 0 0)
            (CallFunction|TurnonDevices)
            (if _istimertoggled
              (Utilities|Time|SetTimerbyFunctionName 0 "TurnOffDevices" _toggletime)
              (Variables|Default|SetCanBeUsed false)
              (goto _label_2)))))
      (else
        (goto _label)))))

(fn ConstructionScript
  (bind _paperflipbook (Variables|Default|GetPaperFlipbook))
  (if (Variables|Default|GetIsOn)
    (Sprite|SetFlipbook _paperflipbook (Variables|Default|GetOnSprite))
    (else
      (Sprite|SetFlipbook _paperflipbook (Variables|Default|GetOffSprite)))))

(fn TurnOffDevices
  (bind _timersounc (Variables|Audio|GetTimerSounc))
  (Variables|Default|SetIsOn false)
  (Sprite|SetFlipbook (Variables|Default|GetPaperFlipbook) (Variables|Default|GetOffSprite))
  (bind _array_element (Utilities|Array|ForEachLoopwithBreak (Variables|Default|GetDevices))
    (:LoopBody
      (Class|IInteractable|TurnOff(Message) _array_element))
    (:Completed
      (Variables|Default|SetCanBeUsed true)
      (Utilities|IsValid _timersounc
        (:Is%20Valid
          (Components|DestroyComponent _timersounc))))))

(fn TurnonDevices
  (bind _timersounc (Variables|Audio|GetTimerSounc))
  (Variables|Default|SetIsOn true)
  (Sprite|SetFlipbook (Variables|Default|GetPaperFlipbook) (Variables|Default|GetOnSprite))
  (bind _array_element (Utilities|Array|ForEachLoopwithBreak (Variables|Default|GetDevices))
    (:LoopBody
      (Class|IInteractable|Turnon(Message) _array_element))
    (:Completed
      (Variables|Default|SetCanBeUsed true)
      (Utilities|IsValid _timersounc
        (:Is%20Valid
          (Components|DestroyComponent _timersounc))))))