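; BP_DoubleDoor is a puzzle double door that swings open and closed through Turnon and TurnOff events.
; Turnon plays a sound and runs the DoorSting timeline, whose alpha lerps the left and right pivot points from a shared starting rotation to their own end rotations.
; TurnOff plays a different sound and reverses the same timeline from its end to close the doors.
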(event EventTurnon
  (bind _startingrotation (Variables|Default|GetStartingRotation))
  (Audio|PlaySoundatLocation "/Game/Static/Audio/Puzzle/Dash_2_Cue.Dash_2_Cue" (Transformation|GetActorLocation) "0, 0, 0" 1.0 1.0 0.0 0 0 0)
  (bind _alpha (Timeline|DoorSting PlayFromStart)
    (:Update
      (Transformation|SetRelativeRotation (Variables|Default|GetRightPivitPoint) (Math|Rotator|Lerp(Rotator) _startingrotation (Variables|Default|GetRightDoorEnd) _alpha) false false)
      (Transformation|SetRelativeRotation (Variables|Default|GetLeftPivitPoint) (Math|Rotator|Lerp(Rotator) _startingrotation (Variables|Default|GetLeftDoorEnd) _alpha) false false))))

(event EventTurnOff
  (bind _startingrotation (Variables|Default|GetStartingRotation))
  (Audio|PlaySoundatLocation "/Game/Static/Audio/Puzzle/Slide_1_Cue.Slide_1_Cue" (Transformation|GetActorLocation) "0, 0, 0" 1.0 1.0 0.0 0 0 0)
  (bind _alpha (Timeline|DoorSting ReverseFromEnd)
    (:Update
      (Transformation|SetRelativeRotation (Variables|Default|GetRightPivitPoint) (Math|Rotator|Lerp(Rotator) _startingrotation (Variables|Default|GetRightDoorEnd) _alpha) false false)
      (Transformation|SetRelativeRotation (Variables|Default|GetLeftPivitPoint) (Math|Rotator|Lerp(Rotator) _startingrotation (Variables|Default|GetLeftDoorEnd) _alpha) false false))))

(fn ConstructionScript)